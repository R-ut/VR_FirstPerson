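; Knife pickup that counts as a piece of real evidence for the first-person character.
; A collision sphere toggles a prompt widget for any overlapping actor and opens or closes a gate when that actor is the player character.
; With input enabled at BeginPlay, pressing E through the open gate increments the player's RealEvidence count and destroys the knife.
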(event `self.ReceiveBeginPlay`
  (bind _asbp_first_person_character (cast `/Game/FirstPerson/Blueprints/BP_FirstPersonCharacter` (`GameplayStatics.GetPlayerCharacter` 0)))
  (set `self.Current Player` _asbp_first_person_character)
  (`self.EnableInput` (`GameplayStatics.GetPlayerController` 0)))

(event `Key|E` :consume false
  (params (Key :type "Key Structure"))
  (bind _returnvalue (`GameplayStatics.GetPlayerCharacter` 0))
  (:`Pressed`
    (`/Engine/EditorBlueprintResources/StandardMacros.Gate` true :!label _label
      (:`Exit`
        (bind _asbp_first_person_character (cast `/Game/FirstPerson/Blueprints/BP_FirstPersonCharacter` _returnvalue))
        (set `/Game/FirstPerson/Blueprints/BP_FirstPersonCharacter.Real Evidence` (+ (`/Game/FirstPerson/Blueprints/BP_FirstPersonCharacter.Real Evidence` (`self.Current Player`)) 1) _asbp_first_person_character)
        (cast `/Game/FirstPerson/Blueprints/BP_FirstPersonCharacter` _returnvalue)
        (`self.K2_DestroyActor`)
        (cast `/Game/FirstPerson/Blueprints/BP_FirstPersonCharacter` _returnvalue)))))

(event `self.Sphere_Coll.OnComponentBeginOverlap`
  (params (OverlappedComponent :type "PrimitiveComponent Object Reference") (OtherActor :type "Actor Object Reference") (OtherComp :type "PrimitiveComponent Object Reference") (OtherBodyIndex :type Integer) (bFromSweep :type Boolean) (SweepResult :type "HitResult Structure (by ref)"))
  (`SceneComponent.SetVisibility` (`self.Widget`) true false)
  (cast `/Game/FirstPerson/Blueprints/BP_FirstPersonCharacter` OtherActor)
  (goto _label :!via `Open`))

(event `self.Sphere_Coll.OnComponentEndOverlap`
  (params (OverlappedComponent :type "PrimitiveComponent Object Reference") (OtherActor :type "Actor Object Reference") (OtherComp :type "PrimitiveComponent Object Reference") (OtherBodyIndex :type Integer))
  (`SceneComponent.SetVisibility` (`self.Widget`) false false)
  (cast `/Game/FirstPerson/Blueprints/BP_FirstPersonCharacter` OtherActor)
  (goto _label :!via `Close`))

(fn `UserConstructionScript`)